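; BP_Fog is a fog actor that switches visibility between Arena and Settore setups, each with a matching sky component.
; Overlapping BoxArena with CharPrinc_Character hides Settore and its sky and shows Arena and its sky.
; The BoxSettore overlap does nothing, and a similar visibility chain that shows SkySettore is left unwired.
; The construction script shows the Arena pair or the Settore pair based on an Arena check, without hiding the other.
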(event OnComponentBeginOverlap(BoxSettore)
  (params (OverlappedComponent :type Primitive%20Component%20Object%20Reference) (OtherActor :type Actor%20Object%20Reference) (OtherComp :type Primitive%20Component%20Object%20Reference) (OtherBodyIndex :type Integer) (bFromSweep :type Boolean) (SweepResult :type Hit%20Result%20Structure%20%28by%20ref%29)))

(event OnComponentBeginOverlap(BoxArena)
  (params (OverlappedComponent :type Primitive%20Component%20Object%20Reference) (OtherActor :type Actor%20Object%20Reference) (OtherComp :type Primitive%20Component%20Object%20Reference) (OtherBodyIndex :type Integer) (bFromSweep :type Boolean) (SweepResult :type Hit%20Result%20Structure%20%28by%20ref%29))
  (Utilities|Casting|CastToCharPrinc_Character OtherActor)
  (Rendering|SetVisibility (Variables|Default|GetSettore) false true)
  (Rendering|SetVisibility (Variables|Default|GetArena) true true)
  (Rendering|SetVisibility (Variables|Default|GetSkyArena) true false)
  (Rendering|SetVisibility (Variables|Default|GetSkySettore) false false))

(fn ConstructionScript
  ;[1 1 1] Collega questo
  (if (Variables|Default|GetArena?)
    (Rendering|SetVisibility (Variables|Default|GetArena) true true)
    (Rendering|SetVisibility (Variables|Default|GetSkyArena) true true)
    (else
      (Rendering|SetVisibility (Variables|Default|GetSettore) true true)
      (Rendering|SetVisibility (Variables|Default|GetSkySettore) true true))))
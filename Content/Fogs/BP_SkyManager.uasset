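; Sky manager that switches a SkyLight between Arena and Settore lighting presets, each defining cubemap, intensity and light color.
; The construction script applies one preset based on the Arena variable.
; At runtime, CharPrinc_Character entering BoxArena applies the Arena preset, while the BoxSettore overlap does nothing, so nothing switches back to Settore.
; Visibility-toggling logic remains in both graphs but is disconnected.
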(event OnComponentBeginOverlap(BoxSettore)
  (params (OverlappedComponent :type Primitive%20Component%20Object%20Reference) (OtherActor :type Actor%20Object%20Reference) (OtherComp :type Primitive%20Component%20Object%20Reference) (OtherBodyIndex :type Integer) (bFromSweep :type Boolean) (SweepResult :type Hit%20Result%20Structure%20%28by%20ref%29)))

(event OnComponentBeginOverlap(BoxArena)
  (params (OverlappedComponent :type Primitive%20Component%20Object%20Reference) (OtherActor :type Actor%20Object%20Reference) (OtherComp :type Primitive%20Component%20Object%20Reference) (OtherBodyIndex :type Integer) (bFromSweep :type Boolean) (SweepResult :type Hit%20Result%20Structure%20%28by%20ref%29))
  (Utilities|Casting|CastToCharPrinc_Character OtherActor)
  (CallFunction|SetArenaSettings))

(event Custom|SetArenaSettings
  (bind _skyarenaproperties (Variables|Default|GetSkyArenaProperties))
  (bind _skylight (Variables|Default|GetSkyLight))
  (bind _lightcomponent (Variables|/Script/Engine.SkyLight|GetLightComponent _skylight))
  (Class|SkyLightComponent|SetCubemap _lightcomponent (.cubemap _skyarenaproperties))
  (Rendering|Components|Light|SetIntensity _lightcomponent (.intensity _skyarenaproperties))
  (Rendering|Components|Light|SetLightColor _lightcomponent (Math|Conversions|ToLinearColor(Color) (.lightcolor _skyarenaproperties))))

(event Custom|SetSettoreSettings
  (bind _skysettoreproperties (Variables|Default|GetSkySettoreProperties))
  (bind _skylight (Variables|Default|GetSkyLight))
  (bind _lightcomponent (Variables|/Script/Engine.SkyLight|GetLightComponent _skylight))
  (Class|SkyLightComponent|SetCubemap _lightcomponent (.cubemap _skysettoreproperties))
  (Rendering|Components|Light|SetIntensity _lightcomponent (.intensity _skysettoreproperties))
  (Rendering|Components|Light|SetLightColor _lightcomponent (Math|Conversions|ToLinearColor(Color) (.lightcolor _skysettoreproperties))))

(fn ConstructionScript
  (if (Variables|Default|GetArena?)
    (CallFunction|SetArenaSettings)
    (else
      (CallFunction|SetSettoreSettings))))
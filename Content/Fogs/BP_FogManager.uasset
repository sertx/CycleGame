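; Fog manager that blends the scene's height fog between presets for three zones: Arena, Settore and Anticamera.
; ChangeFog ignores the current zone, otherwise plays that zone's own timeline, driving height, directional and volumetric fog settings toward its properties.
; Lerps start from live values each update, so blends compound rather than run linearly; Anticamera density instead ramps from zero.
; The volumetric toggle is set directly, and other timelines are never stopped.
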(event Custom|ChangeFog
  (params (ToSettore? :type ENUM_FogStates%20Enum :default "NewEnumerator0"))
  (bind _scenefog (Variables|Default|GetSceneFog))
  (bind _settoreproperties (Variables|Default|GetSettoreProperties))
  (bind _anticameraproperties (Variables|Default|GetAnticameraProperties))
  (bind _arenaproperties (Variables|Default|GetArenaProperties))
  (bind _component (Variables|/Script/Engine.ExponentialHeightFog|GetComponent _scenefog))
  (bind _component_2 (Variables|/Script/Engine.ExponentialHeightFog|GetComponent _scenefog))
  (bind _component_3 (Variables|/Script/Engine.ExponentialHeightFog|GetComponent _scenefog))
  (if (Utilities|Enum|NotEqual(Enum) ToSettore? (Variables|Default|GetCurrentFog))
    (switch Utilities|FlowControl|Switch|SwitchonENUM_FogStates ToSettore?
      (:NewEnumerator0
        (Variables|Default|SetCurrentFog "NewEnumerator0")
        (bind _alpha (Timeline|Timeline_1 PlayFromStart)
          (:Update
            (Utilities|FlowControl|Sequence
              (:then_0
                (Class|ExponentialHeightFogComponent|SetFogDensity _component (Math|Float|Lerp (Variables|/Script/Engine.ExponentialHeightFogComponent|GetFogDensity _component) (.density _arenaproperties) _alpha)))
              (:then_1
                (Class|ExponentialHeightFogComponent|SetFogInscatteringColor _component (Math|Color|Lerp(LinearColor) (Variables|/Script/Engine.ExponentialHeightFogComponent|GetFogInscatteringColor _component) (.color _arenaproperties) _alpha)))
              (:then_2
                (Class|ExponentialHeightFogComponent|SetFogHeightFalloff _component (Math|Float|Lerp (Variables|/Script/Engine.ExponentialHeightFogComponent|GetFogHeightFalloff _component) (.falloff _arenaproperties) _alpha)))
              (:then_3
                (Class|ExponentialHeightFogComponent|SetFogMaxOpacity _component (Math|Float|Lerp (Variables|/Script/Engine.ExponentialHeightFogComponent|GetFogMaxOpacity _component) (.opacity _arenaproperties) _alpha)))
              (:then_4
                (Class|ExponentialHeightFogComponent|SetFogCutoffDistance _component (Math|Float|Lerp (Variables|/Script/Engine.ExponentialHeightFogComponent|GetFogCutoffDistance _component) (.cutoffdistance _arenaproperties) _alpha)))
              (:then_5
                (Class|ExponentialHeightFogComponent|SetDirectionalInscatteringExponent _component (Math|Float|Lerp (Variables|/Script/Engine.ExponentialHeightFogComponent|GetDirectionalInscatteringExponent _component) (.directionalinterscatteringexponent _arenaproperties) _alpha)))
              (:then_6
                (Class|ExponentialHeightFogComponent|SetDirectionalInscatteringColor _component (Math|Color|Lerp(LinearColor) (Variables|/Script/Engine.ExponentialHeightFogComponent|GetDirectionalInscatteringColor _component) (.directionalinterscatteringcolor _arenaproperties) _alpha)))
              (:then_7
                (Class|ExponentialHeightFogComponent|SetVolumetricFog _component (.volumetricfog _arenaproperties)))
              (:then_8
                (Class|ExponentialHeightFogComponent|SetVolumetricFogAlbedo _component (Math|Conversions|ToColor(LinearColor) (Math|Color|Lerp(LinearColor) (Math|Conversions|ToLinearColor(Color) (Variables|/Script/Engine.ExponentialHeightFogComponent|GetVolumetricFogAlbedo _component)) (.albedo _arenaproperties) _alpha))))
              (:then_9
                (Class|ExponentialHeightFogComponent|SetVolumetricFogEmissive _component (Math|Color|Lerp(LinearColor) (Variables|/Script/Engine.ExponentialHeightFogComponent|GetVolumetricFogEmissive _component) (.emissive _arenaproperties) _alpha)))
              (:then_10
                (Class|ExponentialHeightFogComponent|SetVolumetricFogExtinctionScale _component (Math|Float|Lerp (Variables|/Script/Engine.ExponentialHeightFogComponent|GetVolumetricFogExtinctionScale _component) (.extinctionscale _arenaproperties) _alpha)))
              (:then_11
                (Class|ExponentialHeightFogComponent|SetVolumetricFogDistance _component (Math|Float|Lerp (Variables|/Script/Engine.ExponentialHeightFogComponent|GetVolumetricFogDistance _component) (.viewdistance _arenaproperties) _alpha)))
              (:then_12
                (Class|ExponentialHeightFogComponent|SetVolumetricFogScatteringDistribution _component (Math|Float|Lerp (Variables|/Script/Engine.ExponentialHeightFogComponent|GetVolumetricFogScatteringDistribution _component) (.scatteringdistribution _arenaproperties) _alpha)))))))
      (:NewEnumerator1
        (Variables|Default|SetCurrentFog "NewEnumerator1")
        (bind _alpha_2 (Timeline|Transition PlayFromStart)
          (:Update
            (Utilities|FlowControl|Sequence
              (:then_0
                (Class|ExponentialHeightFogComponent|SetFogDensity _component_3 (Math|Float|Lerp (Variables|/Script/Engine.ExponentialHeightFogComponent|GetFogDensity _component_3) (.density _settoreproperties) _alpha_2)))
              (:then_1
                (Class|ExponentialHeightFogComponent|SetFogInscatteringColor _component_3 (Math|Color|Lerp(LinearColor) (Variables|/Script/Engine.ExponentialHeightFogComponent|GetFogInscatteringColor _component_3) (.color _settoreproperties) _alpha_2)))
              (:then_2
                (Class|ExponentialHeightFogComponent|SetFogHeightFalloff _component_3 (Math|Float|Lerp (Variables|/Script/Engine.ExponentialHeightFogComponent|GetFogHeightFalloff _component_3) (.falloff _settoreproperties) _alpha_2)))
              (:then_3
                (Class|ExponentialHeightFogComponent|SetFogMaxOpacity _component_3 (Math|Float|Lerp (Variables|/Script/Engine.ExponentialHeightFogComponent|GetFogMaxOpacity _component_3) (.opacity _settoreproperties) _alpha_2)))
              (:then_4
                (Class|ExponentialHeightFogComponent|SetFogCutoffDistance _component_3 (Math|Float|Lerp (Variables|/Script/Engine.ExponentialHeightFogComponent|GetFogCutoffDistance _component_3) (.cutoffdistance _settoreproperties) _alpha_2)))
              (:then_5
                (Class|ExponentialHeightFogComponent|SetDirectionalInscatteringExponent _component_3 (Math|Float|Lerp (Variables|/Script/Engine.ExponentialHeightFogComponent|GetDirectionalInscatteringExponent _component_3) (.directionalinterscatteringexponent _settoreproperties) _alpha_2)))
              (:then_6
                (Class|ExponentialHeightFogComponent|SetDirectionalInscatteringColor _component_3 (Math|Color|Lerp(LinearColor) (Variables|/Script/Engine.ExponentialHeightFogComponent|GetDirectionalInscatteringColor _component_3) (.directionalinterscatteringcolor _settoreproperties) _alpha_2)))
              (:then_7
                (Class|ExponentialHeightFogComponent|SetVolumetricFog _component_3 (.volumetricfog _settoreproperties)))
              (:then_8
                (Class|ExponentialHeightFogComponent|SetVolumetricFogAlbedo _component_3 (Math|Conversions|ToColor(LinearColor) (Math|Color|Lerp(LinearColor) (Math|Conversions|ToLinearColor(Color) (Variables|/Script/Engine.ExponentialHeightFogComponent|GetVolumetricFogAlbedo _component_3)) (.albedo _settoreproperties) _alpha_2))))
              (:then_9
                (Class|ExponentialHeightFogComponent|SetVolumetricFogEmissive _component_3 (Math|Color|Lerp(LinearColor) (Variables|/Script/Engine.ExponentialHeightFogComponent|GetVolumetricFogEmissive _component_3) (.emissive _settoreproperties) _alpha_2)))
              (:then_10
                (Class|ExponentialHeightFogComponent|SetVolumetricFogExtinctionScale _component_3 (Math|Float|Lerp (Variables|/Script/Engine.ExponentialHeightFogComponent|GetVolumetricFogExtinctionScale _component_3) (.extinctionscale _settoreproperties) _alpha_2)))
              (:then_11
                (Class|ExponentialHeightFogComponent|SetVolumetricFogDistance _component_3 (Math|Float|Lerp (Variables|/Script/Engine.ExponentialHeightFogComponent|GetVolumetricFogDistance _component_3) (.viewdistance _settoreproperties) _alpha_2)))
              (:then_12
                (Class|ExponentialHeightFogComponent|SetVolumetricFogScatteringDistribution _component_3 (Math|Float|Lerp (Variables|/Script/Engine.ExponentialHeightFogComponent|GetVolumetricFogScatteringDistribution _component_3) (.scatteringdistribution _settoreproperties) _alpha_2)))))))
      (:NewEnumerator2
        (Variables|Default|SetCurrentFog "NewEnumerator2")
        (bind _alpha_3 (Timeline|Timeline_0 PlayFromStart)
          (:Update
            (Utilities|FlowControl|Sequence
              (:then_0
                (Class|ExponentialHeightFogComponent|SetFogDensity _component_2 (Math|Float|Lerp 0.0 (.density _anticameraproperties) _alpha_3)))
              (:then_1
                (Class|ExponentialHeightFogComponent|SetFogInscatteringColor _component_2 (Math|Color|Lerp(LinearColor) (Variables|/Script/Engine.ExponentialHeightFogComponent|GetFogInscatteringColor _component_2) (.color _anticameraproperties) _alpha_3)))
              (:then_2
                (Class|ExponentialHeightFogComponent|SetFogHeightFalloff _component_2 (Math|Float|Lerp (Variables|/Script/Engine.ExponentialHeightFogComponent|GetFogHeightFalloff _component_2) (.falloff _anticameraproperties) _alpha_3)))
              (:then_3
                (Class|ExponentialHeightFogComponent|SetFogMaxOpacity _component_2 (Math|Float|Lerp (Variables|/Script/Engine.ExponentialHeightFogComponent|GetFogMaxOpacity _component_2) (.opacity _anticameraproperties) _alpha_3)))
              (:then_4
                (Class|ExponentialHeightFogComponent|SetFogCutoffDistance _component_2 (Math|Float|Lerp (Variables|/Script/Engine.ExponentialHeightFogComponent|GetFogCutoffDistance _component_2) (.cutoffdistance _anticameraproperties) _alpha_3)))
              (:then_5
                (Class|ExponentialHeightFogComponent|SetDirectionalInscatteringExponent _component_2 (Math|Float|Lerp (Variables|/Script/Engine.ExponentialHeightFogComponent|GetDirectionalInscatteringExponent _component_2) (.directionalinterscatteringexponent _anticameraproperties) _alpha_3)))
              (:then_6
                (Class|ExponentialHeightFogComponent|SetDirectionalInscatteringColor _component_2 (Math|Color|Lerp(LinearColor) (Variables|/Script/Engine.ExponentialHeightFogComponent|GetDirectionalInscatteringColor _component_2) (.directionalinterscatteringcolor _anticameraproperties) _alpha_3)))
              (:then_7
                (Class|ExponentialHeightFogComponent|SetVolumetricFog _component_2 (.volumetricfog _anticameraproperties)))
              (:then_8
                (Class|ExponentialHeightFogComponent|SetVolumetricFogAlbedo _component_2 (Math|Conversions|ToColor(LinearColor) (Math|Color|Lerp(LinearColor) (Math|Conversions|ToLinearColor(Color) (Variables|/Script/Engine.ExponentialHeightFogComponent|GetVolumetricFogAlbedo _component_2)) (.albedo _anticameraproperties) _alpha_3))))
              (:then_9
                (Class|ExponentialHeightFogComponent|SetVolumetricFogEmissive _component_2 (Math|Color|Lerp(LinearColor) (Variables|/Script/Engine.ExponentialHeightFogComponent|GetVolumetricFogEmissive _component_2) (.emissive _anticameraproperties) _alpha_3)))
              (:then_10
                (Class|ExponentialHeightFogComponent|SetVolumetricFogExtinctionScale _component_2 (Math|Float|Lerp (Variables|/Script/Engine.ExponentialHeightFogComponent|GetVolumetricFogExtinctionScale _component_2) (.extinctionscale _anticameraproperties) _alpha_3)))
              (:then_11
                (Class|ExponentialHeightFogComponent|SetVolumetricFogDistance _component_2 (Math|Float|Lerp (Variables|/Script/Engine.ExponentialHeightFogComponent|GetVolumetricFogDistance _component_2) (.viewdistance _anticameraproperties) _alpha_3)))
              (:then_12
                (Class|ExponentialHeightFogComponent|SetVolumetricFogScatteringDistribution _component_2 (Math|Float|Lerp (Variables|/Script/Engine.ExponentialHeightFogComponent|GetVolumetricFogScatteringDistribution _component_2) (.scatteringdistribution _anticameraproperties) _alpha_3))))))))))

(fn ConstructionScript)
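; Modular double sliding door, apparently a temporary version, toggled by Interact or driven by trigger overlap when UsesTriggerBox is set.
; Without that flag, leaving the trigger starts a timer that calls Close if no main character remains inside.
; Open uses relative MoveComponentTo offsets, but the right-hand move has no component assigned.
; Close only clears IsOpen without moving the panels; the DoorsMovement timeline logic is disconnected.
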(event OnComponentBeginOverlap(DoorTrigger)
  (params (OverlappedComponent :type Primitive%20Component%20Object%20Reference) (OtherActor :type Actor%20Object%20Reference) (OtherComp :type Primitive%20Component%20Object%20Reference) (OtherBodyIndex :type Integer) (bFromSweep :type Boolean) (SweepResult :type Hit%20Result%20Structure%20%28by%20ref%29))
  (if (Variables|Default|GetUsesTriggerBox)
    (CallFunction|Open)
    (elif (Utilities|Time|IsValidTimerHandle (stale OnComponentEndOverlap(DoorTrigger) _returnvalue))
      (Utilities|Time|InvalidateTimerHandle (stale OnComponentEndOverlap(DoorTrigger) _returnvalue)))))

(event OnComponentEndOverlap(DoorTrigger)
  (params (OverlappedComponent :type Primitive%20Component%20Object%20Reference) (OtherActor :type Actor%20Object%20Reference) (OtherComp :type Primitive%20Component%20Object%20Reference) (OtherBodyIndex :type Integer))
  (if (Variables|Default|GetUsesTriggerBox)
    (CallFunction|Close)
    (else
      (bind _returnvalue (Utilities|Time|SetTimerbyFunctionName 0 "AutomaticClose" 2.0)))))

(event Custom|Open
  (bind _leftdoor (Variables|Default|GetLeftDoor))
  (bind _rightdoor (Variables|Default|GetRightDoor))
  (bind _relativelocation (Variables|/Script/Engine.SceneComponent|GetRelativeLocation _leftdoor))
  (bind _relativelocation_2 (Variables|/Script/Engine.SceneComponent|GetRelativeLocation _rightdoor))
  (if (Variables|Default|GetCanOpen)
    (Variables|Default|SetIsOpen? true)
    (Utilities|FlowControl|Sequence
      (:then_0
        (Components|MoveComponentTo _leftdoor (Math|Vector|MakeVector (+ (.x _relativelocation) -1.4e+02) (.y _relativelocation) (.z _relativelocation)) "0, 0, 0" false false 2.0 false))
      (:then_1
        (Components|MoveComponentTo 0 (Math|Vector|MakeVector (+ (.x _relativelocation_2) 1.4e+02) (.y _relativelocation_2) (.z _relativelocation_2)) "0, 0, 0" false false 2.0 false)))))

(event Custom|Close
  (if (Variables|Default|GetCanOpen)
    (Variables|Default|SetIsOpen? false)))

(event EventInteract
  (if (Variables|Default|GetIsOpen?)
    (CallFunction|Close)
    (else
      (CallFunction|Open))))

(fn ConstructionScript)

(fn AutomaticClose
  (if (not (> (Utilities|Array|Length (Collision|GetOverlappingActors (Variables|Default|GetDoorTrigger) "/Game/Character/CharPrinc_Character.CharPrinc_Character_C" :!class /Script/Engine.PrimitiveComponent)) 0))
    (CallFunction|Close)))
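; BP_DoorKeyhole is a door keyhole that the player can interact with to unlock using picked-up keys.
; Interact casts the player pawn to CharPrinc_Character and, while still locked, checks its key flags against RequiresKey1 and RequiresKey2.
; Success plays the character's key insertion, sets Unlocked and fires CallUnlocked.
; Only the Key2 branch reaches unlocking, so nothing happens when RequiresKey2 is false.
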(event EventInteract
  (bind _aschar_princ_character (Utilities|Casting|CastToCharPrinc_Character (Game|Player|GetPlayerPawn 0)))
  (if (not (Variables|Default|GetUnlocked?))
    (if (Variables|Default|GetRequiresKey1)
      (if (Variables|/Game/Character/CharPrinc_Character.CharPrinc_Character_C|GetKey1PickedUp _aschar_princ_character)
        (if (Variables|Default|GetRequiresKey2) :!label _label
          (if (Variables|/Game/Character/CharPrinc_Character.CharPrinc_Character_C|GetKey2PickedUp _aschar_princ_character)
            (Default|PlayInsertKey _aschar_princ_character)
            (Variables|Default|SetUnlocked? true)
            (Default|CallUnlocked))))
      (else
        (goto _label)))))

(fn ConstructionScript)
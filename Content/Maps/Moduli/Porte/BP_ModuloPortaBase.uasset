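; Base modular double sliding door, opened and closed through Interact or, with UsesTriggerBox, by trigger overlap.
; A timeline slides both panels along X from their BeginPlay positions, with optional open and close sound events.
; Without trigger mode, leaving an open door starts a delayed AutomaticClose, which closes only if no player character overlaps.
; CanOpen gates movement; the construction script uses it for the light material and picks big or small sounds from BigSound.
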(event OnComponentBeginOverlap(DoorTrigger)
  (params (OverlappedComponent :type Primitive%20Component%20Object%20Reference) (OtherActor :type Actor%20Object%20Reference) (OtherComp :type Primitive%20Component%20Object%20Reference) (OtherBodyIndex :type Integer) (bFromSweep :type Boolean) (SweepResult :type Hit%20Result%20Structure%20%28by%20ref%29))
  (if (Variables|Default|GetUsesTriggerBox)
    (CallFunction|Open)
    (elif (Utilities|Time|IsValidTimerHandle (stale OnComponentEndOverlap(DoorTrigger) _returnvalue))
      (Utilities|Time|InvalidateTimerHandle (stale OnComponentEndOverlap(DoorTrigger) _returnvalue)))))

(event OnComponentEndOverlap(DoorTrigger)
  (params (OverlappedComponent :type Primitive%20Component%20Object%20Reference) (OtherActor :type Actor%20Object%20Reference) (OtherComp :type Primitive%20Component%20Object%20Reference) (OtherBodyIndex :type Integer))
  (if (Variables|Default|GetUsesTriggerBox)
    (CallFunction|Close)
    (elif (Variables|Default|GetIsOpen?)
      (bind _returnvalue (Utilities|Time|SetTimerbyFunctionName 0 "AutomaticClose" 2.0)))))

(event Custom|Open
  (bind _leftdoor (Variables|Default|GetLeftDoor))
  (bind _rightdoor (Variables|Default|GetRightDoor))
  (bind _relativelocation (Variables|/Script/Engine.SceneComponent|GetRelativeLocation _leftdoor))
  (bind _relativelocation_2 (Variables|/Script/Engine.SceneComponent|GetRelativeLocation _rightdoor))
  (if (Variables|Default|GetCanOpen)
    (if (not (Audio|Components|Audio|IsPlaying (Variables|Default|GetOpenCloseTL)))
      (Variables|Default|SetIsOpen? true)
      (if (Variables|Default|GetShouldSound?)
        (Class|FMODBlueprintStatics|PlayEventatLocation (Variables|Default|GetOpenEvent) (Transformation|GetActorTransform))
        (bind _distance (Timeline|OpenCloseTL Play)
          (:Update
            (Transformation|SetRelativeLocation _leftdoor (Math|Vector|MakeVector (* (+ (Variables|Default|GetLeftDoorInitialLocation) _distance) -1.0) (.y _relativelocation) (.z _relativelocation)) false false)
            (Transformation|SetRelativeLocation _rightdoor (Math|Vector|MakeVector (+ (Variables|Default|GetRightDoorInitialLocation) _distance) (.y _relativelocation_2) (.z _relativelocation_2)) false false)))
        (else
          (Timeline|OpenCloseTL Play))))))

(event Custom|Close
  (bind _leftdoor (Variables|Default|GetLeftDoor))
  (bind _rightdoor (Variables|Default|GetRightDoor))
  (bind _relativelocation (Variables|/Script/Engine.SceneComponent|GetRelativeLocation _leftdoor))
  (bind _relativelocation_2 (Variables|/Script/Engine.SceneComponent|GetRelativeLocation _rightdoor))
  (if (Variables|Default|GetCanOpen)
    (if (not (Audio|Components|Audio|IsPlaying (Variables|Default|GetOpenCloseTL)))
      (Variables|Default|SetIsOpen? false)
      (if (Variables|Default|GetShouldSound?)
        (Class|FMODBlueprintStatics|PlayEventatLocation (Variables|Default|GetCloseEvent) (Transformation|GetActorTransform))
        (bind _distance (Timeline|OpenCloseTL Reverse)
          (:Update
            (Transformation|SetRelativeLocation _leftdoor (Math|Vector|MakeVector (* (+ (Variables|Default|GetLeftDoorInitialLocation) _distance) -1.0) (.y _relativelocation) (.z _relativelocation)) false false)
            (Transformation|SetRelativeLocation _rightdoor (Math|Vector|MakeVector (+ (Variables|Default|GetRightDoorInitialLocation) _distance) (.y _relativelocation_2) (.z _relativelocation_2)) false false)))
        (else
          (Timeline|OpenCloseTL Reverse))))))

(event Custom|OpenCloseJunction
  (if (Variables|Default|GetIsOpen?)
    (CallFunction|Close)
    (else
      (CallFunction|Open))))

(event EventInteract
  (CallFunction|OpenCloseJunction))

(event EventBeginPlay
  (Variables|Default|SetLeftDoorInitialLocation (.x (Variables|/Script/Engine.SceneComponent|GetRelativeLocation (Variables|Default|GetLeftDoor))))
  (Variables|Default|SetRightDoorInitialLocation (.x (Variables|/Script/Engine.SceneComponent|GetRelativeLocation (Variables|Default|GetRightDoor)))))

(fn ConstructionScript
  (bind _light (Variables|Default|GetLight))
  (if (Variables|Default|GetCanOpen)
    (Rendering|Material|SetMaterial _light 1 "/Game/Master_Material/Texture_Masks/Drone/M_EmissievDoor_Inst.M_EmissievDoor_Inst")
    (else
      (Rendering|Material|SetMaterial _light 1 "/Game/Master_Material/Texture_Masks/Drone/M_EmissievDoor.M_EmissievDoor")))
  (Variables|Default|SetOpenEvent (select (Variables|Default|GetBigSound?) "/Game/FMOD/Events/07_SETTORE_1/doors/doors_open.doors_open" "/Game/FMOD/Events/07_SETTORE_1/doors/doors_piccola_open.doors_piccola_open"))
  (Variables|Default|SetCloseEvent (select (Variables|Default|GetBigSound?) "/Game/FMOD/Events/07_SETTORE_1/doors/doors_close.doors_close" "/Game/FMOD/Events/07_SETTORE_1/doors/doors_piccola_close.doors_piccola_close")))

(fn AutomaticClose
  (if (not (> (Utilities|Array|Length (Collision|GetOverlappingActors (Variables|Default|GetDoorTrigger) "/Game/Character/CharPrinc_Character.CharPrinc_Character_C" :!class /Script/Engine.PrimitiveComponent)) 0))
    (CallFunction|Close)))
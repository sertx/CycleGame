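; Modular sliding double-door actor that opens and closes via its trigger box or an Interact toggle, gated by CanOpen.
; A timeline slides both leaves apart and, after a short delay, reverses on close, with positional open and close sound events.
; With UsesTriggerBox off, leaving the trigger starts a timer that closes the door unless the main character still overlaps it; re-entry invalidates the timer handle.
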(event OnComponentBeginOverlap(DoorTrigger)
  (params (OverlappedComponent :type Primitive%20Component%20Object%20Reference) (OtherActor :type Actor%20Object%20Reference) (OtherComp :type Primitive%20Component%20Object%20Reference) (OtherBodyIndex :type Integer) (bFromSweep :type Boolean) (SweepResult :type Hit%20Result%20Structure%20%28by%20ref%29))
  (if (Variables|Default|GetUsesTriggerBox)
    (CallFunction|Open)
    (elif (Utilities|Time|IsValidTimerHandle (stale OnComponentEndOverlap(DoorTrigger) _returnvalue))
      (Utilities|Time|InvalidateTimerHandle (stale OnComponentEndOverlap(DoorTrigger) _returnvalue)))))

(event OnComponentEndOverlap(DoorTrigger)
  (params (OverlappedComponent :type Primitive%20Component%20Object%20Reference) (OtherActor :type Actor%20Object%20Reference) (OtherComp :type Primitive%20Component%20Object%20Reference) (OtherBodyIndex :type Integer))
  (if (Variables|Default|GetUsesTriggerBox)
    (CallFunction|Close)
    (else
      (bind _returnvalue (Utilities|Time|SetTimerbyFunctionName 0 "AutomaticClose" 2.0)))))

(event Custom|Open
  (bind _leftdoor (Variables|Default|GetLeftDoor))
  (bind _rightdoor (Variables|Default|GetRightDoor))
  (bind _relativelocation (Variables|/Script/Engine.SceneComponent|GetRelativeLocation _leftdoor))
  (bind _relativelocation_2 (Variables|/Script/Engine.SceneComponent|GetRelativeLocation _rightdoor))
  (if (Variables|Default|GetCanOpen)
    (Variables|Default|SetIsOpen? true)
    (Class|FMODBlueprintStatics|PlayEventatLocation "/Game/FMOD/Events/07_SETTORE_1/doors/doors_open.doors_open" (Transformation|GetActorTransform))
    (bind (_direction _distanceright _distanceleft) (Timeline|DoorsMovement Play)
      (:Update
        (Transformation|SetRelativeLocation _leftdoor (Math|Vector|MakeVector _distanceleft (.y _relativelocation) (.z _relativelocation)) false false)
        (Transformation|SetRelativeLocation _rightdoor (Math|Vector|MakeVector _distanceright (.y _relativelocation_2) (.z _relativelocation_2)) false false)))))

(event Custom|Close
  (bind _leftdoor (Variables|Default|GetLeftDoor))
  (bind _rightdoor (Variables|Default|GetRightDoor))
  (bind _relativelocation (Variables|/Script/Engine.SceneComponent|GetRelativeLocation _leftdoor))
  (bind _relativelocation_2 (Variables|/Script/Engine.SceneComponent|GetRelativeLocation _rightdoor))
  (if (Variables|Default|GetCanOpen)
    (Variables|Default|SetIsOpen? false)
    (Class|FMODBlueprintStatics|PlayEventatLocation "/Game/FMOD/Events/07_SETTORE_1/doors/doors_close.doors_close" (Transformation|GetActorTransform))
    (Utilities|FlowControl|Delay 0.3)
    (bind (_direction _distanceright _distanceleft) (Timeline|DoorsMovement Reverse)
      (:Update
        (Transformation|SetRelativeLocation _leftdoor (Math|Vector|MakeVector _distanceleft (.y _relativelocation) (.z _relativelocation)) false false)
        (Transformation|SetRelativeLocation _rightdoor (Math|Vector|MakeVector _distanceright (.y _relativelocation_2) (.z _relativelocation_2)) false false)))))

(event EventInteract
  (if (Variables|Default|GetIsOpen?)
    (CallFunction|Close)
    (else
      (CallFunction|Open))))

(event EventBeginPlay)

(fn ConstructionScript)

(fn AutomaticClose
  (if (not (> (Utilities|Array|Length (Collision|GetOverlappingActors (Variables|Default|GetDoorTrigger) "/Game/Character/CharPrinc_Character.CharPrinc_Character_C" :!class /Script/Engine.PrimitiveComponent)) 0))
    (CallFunction|Close)))
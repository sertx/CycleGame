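; Elevator Blueprint that raises its Platform component by HeightToTravel in a single one-way trip until reset.
; GoUp latches an Activated flag, waits briefly, plays a 2D FMOD elevator sound, then eases the platform upward with MoveComponentTo and flips IsUp.
; Reset clears both flags and snaps the platform to a hard-coded starting height, allowing another ride.
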(event Custom|GoUp
  (bind _platform (Variables|Default|GetPlatform))
  (bind _relativelocation (Variables|/Script/Engine.SceneComponent|GetRelativeLocation _platform))
  (if (and (not (Variables|Default|GetIsUp?)) (not (Variables|Default|GetActivated)))
    (Variables|Default|SetActivated true)
    (Utilities|FlowControl|Delay 0.4)
    (Class|FMODBlueprintStatics|PlayEvent2D "/Game/FMOD/Events/09_ASCENSORE/elevator.elevator")
    (Components|MoveComponentTo _platform (Math|Vector|MakeVector (.x _relativelocation) (.y _relativelocation) (+ (.z _relativelocation) (* (Variables|Default|GetHeightToTravel) (select (Variables|Default|GetIsUp?) -1.0 1.0)))) "0, 0, 0" true true 15.0 false)
    (Variables|Default|SetIsUp? (not (Variables|Default|GetIsUp?)))))

(event Custom|Reset
  (bind _platform (Variables|Default|GetPlatform))
  (bind _relativelocation (Variables|/Script/Engine.SceneComponent|GetRelativeLocation _platform))
  (Variables|Default|SetIsUp? false)
  (Variables|Default|SetActivated false)
  (Transformation|SetRelativeLocation _platform (Math|Vector|MakeVector (.x _relativelocation) (.y _relativelocation) 9.0) false false))

(fn ConstructionScript)
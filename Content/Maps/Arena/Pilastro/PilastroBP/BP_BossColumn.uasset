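; BP_BossColumn is an arena column with a button that powers up the player and activates a floor trap.
; An overlap on BoxFront by Asparaking_Character in a specific AnimState triggers it once, guarded by the Activated flag.
; Button1 animates in and back out with MoveComponentTo, then the character's PowerUp runs and the TRAP_AzotoArena in the FloorTraps child actor is activated.
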(event OnComponentBeginOverlap(BoxFront)
  (params (OverlappedComponent :type Primitive%20Component%20Object%20Reference) (OtherActor :type Actor%20Object%20Reference) (OtherComp :type Primitive%20Component%20Object%20Reference) (OtherBodyIndex :type Integer) (bFromSweep :type Boolean) (SweepResult :type Hit%20Result%20Structure%20%28by%20ref%29))
  (bind _button1 (Variables|Default|GetButton1))
  (bind _relativelocation (Variables|/Script/Engine.SceneComponent|GetRelativeLocation _button1))
  (bind _asasparaking_character (Utilities|Casting|CastToAsparaking_Character OtherActor))
  (if (and (Utilities|Enum|Equal(Enum) (Variables|/Game/Asparaking/Asparaking_Character.Asparaking_Character_C|GetAnim_State _asasparaking_character) "NewEnumerator2") (not (Variables|Default|GetActivated?)))
    (Components|MoveComponentTo _button1 (Math|Vector|MakeVector (.x _relativelocation) (- (.y _relativelocation) 25.0) (.z _relativelocation)) "0, 0, 0" false false 0.3 false)
    (Utilities|FlowControl|Delay 0.2)
    (Components|MoveComponentTo _button1 (Math|Vector|MakeVector (.x _relativelocation) (+ (.y _relativelocation) 25.0) (.z _relativelocation)) "0, 0, 0" true false 0.3 false)
    (Default|PowerUp _asasparaking_character)
    (Variables|Default|SetActivated? true)
    (bind _astrap_azoto_arena (Utilities|Casting|CastToTRAP_AzotoArena (Variables|/Script/Engine.ChildActorComponent|GetChildActor (Variables|Default|GetFloorTraps))))
    (Default|Activate _astrap_azoto_arena)))

(fn ConstructionScript)
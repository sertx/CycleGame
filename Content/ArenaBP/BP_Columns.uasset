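; BP_Columns is an arena column actor that powers up the referenced BestiaTemp when one of its three collision boxes is overlapped.
; Each box's begin-overlap event calls SetActive false on that box, then fires the shared HitColumn event, which calls PowerUp.
; The Asparaking_Character casts never run on the overlap path, so overlaps are not filtered by actor type and HitColumn ignores its character parameter.
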(event OnComponentBeginOverlap(CollBox1)
  (params (OverlappedComponent :type Primitive%20Component%20Object%20Reference) (OtherActor :type Actor%20Object%20Reference) (OtherComp :type Primitive%20Component%20Object%20Reference) (OtherBodyIndex :type Integer) (bFromSweep :type Boolean) (SweepResult :type Hit%20Result%20Structure%20%28by%20ref%29))
  (Components|Activation|SetActive (Variables|Default|GetCollBox1) false false)
  (CallFunction|HitColumn (stale _asasparaking_character)))

(event OnComponentBeginOverlap(CollBox2)
  (params (OverlappedComponent :type Primitive%20Component%20Object%20Reference) (OtherActor :type Actor%20Object%20Reference) (OtherComp :type Primitive%20Component%20Object%20Reference) (OtherBodyIndex :type Integer) (bFromSweep :type Boolean) (SweepResult :type Hit%20Result%20Structure%20%28by%20ref%29))
  (Components|Activation|SetActive (Variables|Default|GetCollBox2) false false)
  (CallFunction|HitColumn (stale _asasparaking_character)))

(event OnComponentBeginOverlap(CollBox3)
  (params (OverlappedComponent :type Primitive%20Component%20Object%20Reference) (OtherActor :type Actor%20Object%20Reference) (OtherComp :type Primitive%20Component%20Object%20Reference) (OtherBodyIndex :type Integer) (bFromSweep :type Boolean) (SweepResult :type Hit%20Result%20Structure%20%28by%20ref%29))
  (Components|Activation|SetActive (Variables|Default|GetCollBox3) false false)
  (CallFunction|HitColumn (stale _asasparaking_character)))

(event Custom|HitColumn
  (params (Asparaking :type Asparaking%20Character%20Object%20Reference))
  (Default|PowerUp (Variables|Default|GetBestiaTemp)))

(fn ConstructionScript)
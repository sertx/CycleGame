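; BP_WallCamera is a wall camera prop that turns to follow the first player's pawn.
; Each Tick, if that pawn is valid, it sets the Arm's world rotation to the full look-at rotation from the actor's location to the pawn, with no smoothing or limits.
; A disconnected node that would apply only yaw to the Eye never runs, and the construction script is empty.
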(event EventTick
  (params (DeltaSeconds :type Float%20%28single-precision%29))
  (bind _returnvalue (Game|Player|GetPlayerPawn 0))
  (bind _self self)
  (bind _returnvalue_2 (Transformation|GetActorLocation _returnvalue))
  (bind _returnvalue_3 (Transformation|GetActorLocation _self))
  (bind _returnvalue_4 (Math|Rotator|FindLookatRotation _returnvalue_3 _returnvalue_2))
  (if (Utilities|IsValid _returnvalue)
    (Transformation|SetWorldRotation (Variables|Default|GetArm) (Math|Rotator|MakeRotator (.roll _returnvalue_4) (.pitch _returnvalue_4) (.yaw _returnvalue_4)) false false)))

(fn ConstructionScript)
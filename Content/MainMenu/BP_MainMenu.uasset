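; 3D main menu actor presenting Play, Episodes, Options, Stats, Extra and Customize pages as widget capsules on a sliding tray.
; CharPrinc_Controller events step the tray between pages and enter or exit focus, moving the camera and opening the Customize capsule.
; The Play page triggers LowerCapsule, which stops music, opens Botola, lowers the capsule and plays the GameMode cinematic.
; Mouse-drag scrolling is disconnected; SetPlayerCustomizations is empty.
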(event Custom|SelectVoice
  (bind _focuscampos (Variables|Default|GetFocusCamPos))
  (bind _returnvalue (Transformation|GetRelativeTransform _focuscampos))
  ;[1 1 1] Enter and Exit Focus
  (if (not (Variables|Default|GetInFocus))
    (bind _asmain_menu_capsule_page (Utilities|Casting|CastToMainMenu_CapsulePage (UserInterface|GetUserWidgetObject (.Value (Utilities|Map|Find (Variables|Default|GetPagesDict) (Utilities|String|ToString(Text) (Variables|Default|GetCurrentPage)))))))
    (Default|Initialise _asmain_menu_capsule_page)
    (if (Utilities|Enum|Equal(Enum) (Variables|Default|GetCurrentPage) (Utilities|Text|MakeLiteralText "Customize"))
      (bind _asbp_main_capsule (Utilities|Casting|CastToBP_MainCapsule (Variables|/Script/Engine.ChildActorComponent|GetChildActor (Variables|Default|GetCustomizeCapsule))))
      (Default|Open _asbp_main_capsule)
      (else
        (Class|FMODBlueprintStatics|PlayEvent2D "/Game/FMOD/Events/00_MENU/menu_select.menu_select")))
    (Default|SwitchFocus _asmain_menu_capsule_page true)
    (Variables|Default|SetInFocus true)
    (Components|MoveComponentTo (Variables|Default|GetCamera) (.location _returnvalue) (.rotation _returnvalue) false false 1.0 false)))

(event Custom|MoveLeftRight
  (params (Key :type Key%20Structure))
  (if (or (== Key "A") (== Key "Left"))
    (CallFunction|MoveLeft)
    (else
      (CallFunction|MoveRight))))

(event Custom|MoveRight
  (bind _mainpages (Variables|Default|GetMainPages))
  (bind _capsulestray (Variables|Default|GetCapsulesTray))
  (bind _returnvalue (Transformation|GetRelativeTransform _capsulestray))
  ;[1 1 1] Move Left and Right
  (if (not (Math|Boolean|ORBoolean (== (Utilities|Array|LastIndex _mainpages) (Utilities|Array|FindItem _mainpages (Variables|Default|GetCurrentPage))) (Variables|Default|GetIsMoving) (Variables|Default|GetInFocus)))
    (Class|FMODBlueprintStatics|PlayEvent2D "/Game/FMOD/Events/00_MENU/menu_switch.menu_switch")
    (Variables|Default|SetCurrentPage (Utilities|Array|Get(acopy) _mainpages (+ (Utilities|Array|FindItem _mainpages (Variables|Default|GetCurrentPage)) 1)))
    (Variables|Default|SetIsMoving true)
    (Components|MoveComponentTo _capsulestray (Math|Vector|MakeVector (.x (.location _returnvalue)) (- (.y (.location _returnvalue)) 3e+02) (.z (.location _returnvalue))) (.rotation _returnvalue) true true 0.7 false)
    (Variables|Default|SetIsMoving false)))

(event Custom|LowerCapsule
  (bind _flycampos (Variables|Default|GetFlyCamPos))
  (bind _play (Variables|Default|GetPlay))
  (bind _returnvalue (Transformation|GetRelativeTransform _flycampos))
  (bind _relativelocation (Variables|/Script/Engine.SceneComponent|GetRelativeLocation _play))
  (Variables|Default|SetSpawned true)
  (Class|FMODBlueprintStatics|PlayEvent2D "/Game/FMOD/Events/00_MENU/menu_play.menu_play")
  ;[1 1 1] Lower Capsule and Start Game
  (Class|FMODBlueprintStatics|EventInstanceStop (Variables|Default|GetMenuMusic))
  (CallFunction|SetPlayerCustomizations)
  (Utilities|FlowControl|Delay 1.0)
  (Default|OpenCloseJunction (Variables|Default|GetBotola))
  (Utilities|FlowControl|Sequence
    (:then_0
      (Utilities|FlowControl|Delay 3.0)
      (Components|MoveComponentTo _play (Math|Vector|MakeVector (.x _relativelocation) (.y _relativelocation) (- (.z _relativelocation) 6e+02)) "0, 0, 0" false false 6.0 false))
    (:then_1
      (Utilities|FlowControl|Sequence
        (:then_0
          (Default|PlayCinematic (Variables|Default|GetGameMode) true)
          (Utilities|FlowControl|Delay 5.0)
          (Transformation|SetRelativeLocation (Variables|Default|GetPlay) "0, 0, 0" false false)
          (Components|MoveComponentTo (Variables|Default|GetCamera) (.location _returnvalue) (.rotation _returnvalue) false false 0.0 false))))))

(event Custom|MoveLeft
  (bind _mainpages (Variables|Default|GetMainPages))
  (bind _capsulestray (Variables|Default|GetCapsulesTray))
  (bind _returnvalue (Transformation|GetRelativeTransform _capsulestray))
  ;[1 1 1] Move Left and Right
  (if (not (Math|Boolean|ORBoolean (== (Utilities|Array|FindItem _mainpages (Variables|Default|GetCurrentPage)) 0) (Variables|Default|GetIsMoving) (Variables|Default|GetInFocus)))
    (Class|FMODBlueprintStatics|PlayEvent2D "/Game/FMOD/Events/00_MENU/menu_switch.menu_switch")
    (Variables|Default|SetCurrentPage (Utilities|Array|Get(acopy) _mainpages (- (Utilities|Array|FindItem _mainpages (Variables|Default|GetCurrentPage)) 1)))
    (Variables|Default|SetIsMoving true)
    (Components|MoveComponentTo _capsulestray (Math|Vector|MakeVector (.x (.location _returnvalue)) (+ (.y (.location _returnvalue)) 3e+02) (.z (.location _returnvalue))) (.rotation _returnvalue) true true 0.7 false)
    (Variables|Default|SetIsMoving false)))

(event Custom|ExitVoice
  (bind _flycampos (Variables|Default|GetFlyCamPos))
  (bind _returnvalue (Transformation|GetRelativeTransform _flycampos))
  (if (Variables|Default|GetInFocus)
    ;[1 1 1] Enter and Exit Focus
    (if (Utilities|Enum|Equal(Enum) (Variables|Default|GetCurrentPage) (Utilities|Text|MakeLiteralText "Customize"))
      (bind _asbp_main_capsule (Utilities|Casting|CastToBP_MainCapsule (Variables|/Script/Engine.ChildActorComponent|GetChildActor (Variables|Default|GetCustomizeCapsule))))
      (Default|Close _asbp_main_capsule)
      (else
        (Class|FMODBlueprintStatics|PlayEvent2D "/Game/FMOD/Events/00_MENU/menu_back.menu_back")))
    (Variables|Default|SetInFocus false)
    (bind _asmain_menu_capsule_page (Utilities|Casting|CastToMainMenu_CapsulePage (UserInterface|GetUserWidgetObject (.Value (Utilities|Map|Find (Variables|Default|GetPagesDict) (Utilities|String|ToString(Text) (Variables|Default|GetCurrentPage)))))))
    (Default|SwitchFocus _asmain_menu_capsule_page false)
    (Components|MoveComponentTo (Variables|Default|GetCamera) (.location _returnvalue) (.rotation _returnvalue) false false 1.0 false)))

(event Custom|DragTray
  (params (Axis%20Value :type Float%20%28single-precision%29)))

(event EventBeginPlay
  (bind _returnvalue (Game|GetPlayerController 0))
  ;[1 1 1] Initial Setup
  (Utilities|FlowControl|Sequence
    (:then_0
      (Variables|/Script/Engine.PlayerController|SetbShowMouseCursor _returnvalue true)
      (Input|SetInputModeGameandUI _returnvalue 0 "DoNotLock" false))
    (:then_1
      (bind _aschar_princ_controller (Utilities|Casting|CastToCharPrinc_Controller _returnvalue))
      (EventDispatchers|BindEventtoControlledSelectMenuVoice _aschar_princ_controller (delegate Custom|SelectVoice))
      (EventDispatchers|BindEventtoControllerMenuLeftRight _aschar_princ_controller (delegate Custom|MoveLeftRight))
      (EventDispatchers|BindEventtoControllerMenuExitVoice _aschar_princ_controller (delegate Custom|ExitVoice))
      (EventDispatchers|BindEventtoMouseX _aschar_princ_controller (delegate Custom|DragTray)))
    (:then_3
      (Variables|Default|SetCurrentPage (Utilities|Array|Get(acopy) (Variables|Default|GetMainPages))))
    (:then_4
      (CallFunction|SetWidgets))
    (:then_5
      (bind _asthird_person_game_mode (Utilities|Casting|CastToThirdPersonGameMode (Game|GetGameMode)))
      (Variables|Default|SetGameMode _asthird_person_game_mode))
    (:then_6
      (Transformation|SetRelativeLocation (Variables|Default|GetCamera) (Variables|/Script/Engine.SceneComponent|GetRelativeLocation (Variables|Default|GetFlyCamPos)) false false))
    (:then_7
      (bind _aschar_menu_char (Utilities|Casting|CastToChar_MenuChar (Variables|/Script/Engine.ChildActorComponent|GetChildActor (Variables|Default|GetChar))))
      (Variables|/Game/Character/CharPrinc_AnimBP.CharPrinc_AnimBP_C|SetPlayInitialCinematic (Variables|/Game/Character/Char_MenuChar.Char_MenuChar_C|GetAnimInstance _aschar_menu_char) true)
      (Variables|/Game/Character/CharPrinc_AnimBP.CharPrinc_AnimBP_C|SetPlayRate (Variables|/Game/Character/Char_MenuChar.Char_MenuChar_C|GetAnimInstance _aschar_menu_char) 0.0)
      (bind _asmain_menu_customize_widget (Utilities|Casting|CastToMainMenu_CustomizeWidget (UserInterface|GetUserWidgetObject (Variables|Default|GetCustomizeWidget))))
      (Variables|/Game/MainMenu/MainMenu_CustomizeWidget.MainMenu_CustomizeWidget_C|SetPlayer _asmain_menu_customize_widget _aschar_menu_char))
    (:then_8
      (bind _asmain_menu_play_page (Utilities|Casting|CastToMainMenu_PlayPage (UserInterface|GetUserWidgetObject (Variables|Default|GetPlayWidget))))
      (EventDispatchers|BindEventtoPlay _asmain_menu_play_page (delegate Custom|LowerCapsule)))
    (:then_9
      (bind _returnvalue_2 (Class|FMODBlueprintStatics|PlayEvent2D "/Game/FMOD/Events/04_MUSIC/music_menu.music_menu"))
      (Variables|Default|SetMenuMusic _returnvalue_2))))

(event Input|MouseEvents|LeftMouseButton
  (params (Key :type Key%20Structure))
  (:Pressed
    (Variables|Default|SetDragging true))
  (:Released
    (Variables|Default|SetDragging false)
    (bind _alpha (Timeline|Decelerate PlayFromStart)
      (:Update
        (Transformation|AddWorldOffset (Variables|Default|GetCapsulesTray) (Math|Vector|MakeVector (* (Math|Float|Lerp (Variables|Default|GetMouseSpeed) 0.0 _alpha) 4.0) 0.0 0.0) false false)))))

(fn ConstructionScript
  (bind _pagesdict (Variables|Default|GetPagesDict))
  (Utilities|Map|Add _pagesdict "Play" (Variables|Default|GetPlayWidget))
  (Utilities|Map|Add _pagesdict "Episodes" 0)
  (Utilities|Map|Add _pagesdict "Options" (Variables|Default|GetOptionsWidgets))
  (Utilities|Map|Add _pagesdict "Stats" (Variables|Default|GetStatsWidget))
  (Utilities|Map|Add _pagesdict "Extra" (Variables|Default|GetExtraWidget))
  (Utilities|Map|Add _pagesdict "Customize" (Variables|Default|GetCustomizeWidget)))

(fn SetWidgets
  (bind _asmain_menu_capsule_title (Utilities|Casting|CastToMainMenu_CapsuleTitle (UserInterface|GetUserWidgetObject (Variables|Default|GetPlayTitle))))
  (Default|SetTitle _asmain_menu_capsule_title "Play")
  (bind _asmain_menu_capsule_title_2 (Utilities|Casting|CastToMainMenu_CapsuleTitle (UserInterface|GetUserWidgetObject (Variables|Default|GetEpisodesTitle))))
  (Default|SetTitle _asmain_menu_capsule_title_2 "My Episodes")
  (bind _asmain_menu_capsule_title_3 (Utilities|Casting|CastToMainMenu_CapsuleTitle (UserInterface|GetUserWidgetObject (Variables|Default|GetOptionsTitle))))
  (Default|SetTitle _asmain_menu_capsule_title_3 "Options")
  (bind _asmain_menu_capsule_title_4 (Utilities|Casting|CastToMainMenu_CapsuleTitle (UserInterface|GetUserWidgetObject (Variables|Default|GetStatsTitle))))
  (Default|SetTitle _asmain_menu_capsule_title_4 "Stats")
  (bind _asmain_menu_capsule_title_5 (Utilities|Casting|CastToMainMenu_CapsuleTitle (UserInterface|GetUserWidgetObject (Variables|Default|GetExtraTitle))))
  (Default|SetTitle _asmain_menu_capsule_title_5 "Extra")
  (bind _asmain_menu_capsule_title_6 (Utilities|Casting|CastToMainMenu_CapsuleTitle (UserInterface|GetUserWidgetObject (Variables|Default|GetCustomizeTitle))))
  (Default|SetTitle _asmain_menu_capsule_title_6 "Customize"))

(fn SetPlayerCustomizations)
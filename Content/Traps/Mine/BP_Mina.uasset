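; BP_Mina is a reusable mine trap that slows the player character when it enters the trigger Sphere.
; On overlap it casts to CharPrinc_Character, then plays a beep, followed after short delays by explosion FX and sound and a call to Rallentato with speed, duration and play-rate values.
; A DoOnce blocks retriggering and resets after a delay, so the mine re-arms.
; An FMOD PlayEventAtLocation node is left unconnected.
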(event OnComponentBeginOverlap(Sphere)
  (params (OverlappedComponent :type Primitive%20Component%20Object%20Reference) (OtherActor :type Actor%20Object%20Reference) (OtherComp :type Primitive%20Component%20Object%20Reference) (OtherBodyIndex :type Integer) (bFromSweep :type Boolean) (SweepResult :type Hit%20Result%20Structure%20%28by%20ref%29))
  (bind _aschar_princ_character (Utilities|Casting|CastToCharPrinc_Character OtherActor))
  (Utilities|FlowControl|DoOnce false :!label _label
    (:Completed
      (Utilities|FlowControl|Sequence
        (:then_0
          (Class|FMODAudioComponent|Play (Variables|Default|GetBip))
          (Utilities|FlowControl|Delay 0.2)
          (Components|Activation|Activate (Variables|Default|GetFX) true)
          (Class|FMODAudioComponent|Play (Variables|Default|GetExplosion))
          (Utilities|FlowControl|Delay 0.2)
          (Default|Rallentato _aschar_princ_character (Variables|Default|GetNew%20Speed) (Variables|Default|GetDuration) (Variables|Default|GetSlowedPlayRate)))
        (:then_1
          (Utilities|FlowControl|Delay 1.5)
          (goto _label Reset))))))

(event EventBeginPlay)

(fn ConstructionScript)
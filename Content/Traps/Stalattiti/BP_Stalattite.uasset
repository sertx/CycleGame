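; Stalactite trap that drops a cone when the player character enters its trigger collider.
; The overlap halves global time dilation and plays the FallDown timeline, which drives the cone's absolute world Z and restores normal time when finished.
; If moving the cone hits the character, it switches them to ragdoll with a death type and snaps their mesh onto the cone.
; A switch on DodgeLeft follows but has no connected actions.
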(event OnComponentBeginOverlap(Collider)
  (params (OverlappedComponent :type Primitive%20Component%20Object%20Reference) (OtherActor :type Actor%20Object%20Reference) (OtherComp :type Primitive%20Component%20Object%20Reference) (OtherBodyIndex :type Integer) (bFromSweep :type Boolean) (SweepResult :type Hit%20Result%20Structure%20%28by%20ref%29))
  (bind _cone (Variables|Default|GetCone))
  (bind _returnvalue (Transformation|GetWorldLocation _cone))
  (Utilities|Casting|CastToCharPrinc_Character OtherActor)
  (Utilities|Time|SetGlobalTimeDilation 0.5)
  (Utilities|FlowControl|Sequence
    (:then_0
      (bind _fall (Timeline|FallDown Play)
        (:Update
          (bind _sweephitresult (Transformation|SetWorldLocation _cone (Math|Vector|MakeVector (.x _returnvalue) (.y _returnvalue) _fall) false false))
          (bind _aschar_princ_character (Utilities|Casting|CastToCharPrinc_Character (.HitActor (Collision|BreakHitResult _sweephitresult))))
          (Default|ChangeRagdollState _aschar_princ_character true 0.0 "NewEnumerator0")
          (Transformation|AttachComponentToComponent (Variables|/Script/Engine.Character|GetMesh _aschar_princ_character) (Variables|Default|GetCone) "None" "SnapToTarget" "SnapToTarget" "SnapToTarget" true))
        (:Finished
          (Utilities|Time|SetGlobalTimeDilation 1.0))))
    (:then_1
      (switch Utilities|FlowControl|Switch|SwitchonSlattiteDodges (Variables|Default|GetDodgeLeft?)))))

(fn ConstructionScript)